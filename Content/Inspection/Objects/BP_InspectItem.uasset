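; BP_InspectItem is an interactable item actor that hands over its model when grabbed, then removes itself from the world.
; The construction script applies the ItemModel variable to the StaticObject mesh component.
; InteractItem prints a debug message, calls DestroyItem and returns ItemModel to the caller.
; DestroyItem is a custom event that destroys the actor after a short delay.
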(event Custom|Destroy%20Item
  (Utilities|FlowControl|Delay 0.2)
  (Actor|DestroyActor))

(event EventBeginPlay)

(event Collision|EventActorBeginOverlap
  (params (OtherActor :type Actor%20Object%20Reference)))

(event EventTick
  (params (DeltaSeconds :type Float%20%28single-precision%29)))

(fn ConstructionScript
  (Components|StaticMesh|SetStaticMesh (Variables|Default|GetStaticObject) (Variables|Default|GetItemModel)))

(fn InteractItem
  (Development|PrintString "Item Grab")
  (CallFunction|DestroyItem)
  (return (Variables|Default|GetItemModel)))